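; Enemy character that spots the player, fires targeted magic bullets and shows a health bar.
; A damage system component handles health, with its events updating the bar, granting brief invincibility on hit and destroying the actor on death.
; Pawn sensing sets a blackboard seen-player flag that a retriggerable delay clears once sightings stop.
; AttackPlayer sphere-traces forward and, on hitting the player, spawns a bullet at them after a delay.
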(event OnSeePawn(PawnSensing)
  (params (Pawn :type Pawn%20Object%20Reference))
  (bind _returnvalue (Utilities|Name|MakeLiteralName "hasSeenPlayer"))
  (bind _self self)
  (bind _returnvalue_2 (AI|GetAIController _self))
  (bind _returnvalue_3 (AI|GetBlackboard _returnvalue_2))
  (Utilities|FlowControl|Sequence
    (:then_0
      (Utilities|Casting|CastTowheelman_character Pawn)
      (AI|Components|Blackboard|SetValueasBool _returnvalue_3 _returnvalue true))
    (:then_1
      (Utilities|FlowControl|RetriggerableDelay 0.2)
      (AI|Components|Blackboard|SetValueasBool _returnvalue_3 _returnvalue false))))

(event Custom|Death
  (Actor|DestroyActor))

(event Custom|Blocked
  (params (CanBeParried :type Boolean))
  (Development|PrintString "Blocked"))

(event Custom|DamageResponse
  (params (DamageResponse :type E_DamageResponses%20Enum :default "NewEnumerator0"))
  (Development|PrintString (Utilities|String|EnumtoString DamageResponse)))

(event Custom|Attack%20Player
  (bind _returnvalue (Transformation|GetActorLocation))
  (bind _self self)
  (bind _outactors (Actor|GetAllActorsOfClass "/Game/Characters/Enemy/bullet.bullet_C"))
  (bind (_outhit _returnvalue_2) (Collision|SphereTraceForObjects _returnvalue (+ _returnvalue (* (Math|Vector|GetForwardVector (Transformation|GetActorRotation)) 1e+03)) 1.2e+02 (Utilities|Array|MakeArray "ObjectTypeQuery3") false _outactors "None"))
  (if _returnvalue_2
    (bind _aswheelman_character (Utilities|Casting|CastTowheelman_character (.HitActor (Collision|BreakHitResult _outhit))))
    (Utilities|FlowControl|Delay 2.0)
    (Game|SpawnActorfromClass "/Game/Characters/Enemy/BP_magicBullet.BP_magicBullet_C" (Transformation|GetWorldTransform (Variables|Default|GetArrow1 _self)) "Undefined" "MultiplyWithRoot" _self _aswheelman_character 1e+03 true 0)
    (else
      (Development|PrintString "not detected"))))

(event Custom|BeHitted
  (bind _bpc_damagesystem (Variables|Default|GetBPC_DamageSystem))
  (CallFunction|UpdateHealthBar)
  (Variables|/Game/DamageSystem/BPC_DamageSystem.BPC_DamageSystem_C|SetIsInvincible _bpc_damagesystem true)
  (Utilities|FlowControl|Delay 0.5)
  (Variables|/Game/DamageSystem/BPC_DamageSystem.BPC_DamageSystem_C|SetIsInvincible _bpc_damagesystem false))

(event EventBeginPlay
  (CallFunction|UpdateHealthBar))

(fn ConstructionScript
  (bind _bpc_damagesystem (Variables|Default|GetBPC_DamageSystem))
  (EventDispatchers|BindEventtoOnDeath _bpc_damagesystem (EventDispatchers|CreateEvent :!event Custom|Death))
  (EventDispatchers|BindEventtoOnBlocked _bpc_damagesystem (EventDispatchers|CreateEvent :!event Custom|Blocked))
  (EventDispatchers|BindEventtoOnDamageResponse _bpc_damagesystem (EventDispatchers|CreateEvent :!event Custom|DamageResponse))
  (EventDispatchers|BindEventtoBeHitted _bpc_damagesystem (EventDispatchers|CreateEvent :!event Custom|BeHitted)))

(fn UpdateHealthBar
  (bind _bpc_damagesystem (Variables|Default|GetBPC_DamageSystem))
  (bind _asbp_enemy_health (Utilities|Casting|CastToBP_enemyHealth (UserInterface|GetUserWidgetObject (Variables|Default|GethealthBar))))
  (Variables|/Game/UI/BP_enemyHealth.BP_enemyHealth_C|SetHealthPercent _asbp_enemy_health (/ (Variables|/Game/DamageSystem/BPC_DamageSystem.BPC_DamageSystem_C|GetHealth _bpc_damagesystem) (Variables|/Game/DamageSystem/BPC_DamageSystem.BPC_DamageSystem_C|GetMaxHealth _bpc_damagesystem)))
  (return))

(fn GetCurrentHealth
  (return (Variables|/Game/DamageSystem/BPC_DamageSystem.BPC_DamageSystem_C|GetHealth (Variables|Default|GetBPC_DamageSystem))))

(fn GetMaxHealth
  (return (Variables|/Game/DamageSystem/BPC_DamageSystem.BPC_DamageSystem_C|GetMaxHealth (Variables|Default|GetBPC_DamageSystem))))

(fn Heal
  (params (Amount :type Float%20%28double-precision%29))
  (bind _newhealth (CallFunction|Heal Amount))
  (return _newhealth))

(fn TakeDamage
  (params (DamageInfo :type S%20Damage%20Info%20Structure))
  (bind _wasdamaged (Default|TakeDamage (Variables|Default|GetBPC_DamageSystem) DamageInfo))
  (return _wasdamaged))